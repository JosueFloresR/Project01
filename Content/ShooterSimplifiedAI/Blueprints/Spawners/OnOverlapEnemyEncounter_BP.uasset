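; Trigger volume Blueprint that spawns a configured enemy encounter when the player character enters its box.
; The first player overlap passes a DoOnce, plays a 2D spawn sound and waits briefly.
; It then loops over the EnemyStructure array, spawning each enemy class at its spawn point and passing in that entry's behavior tree, assault path and weapon type.
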(event OnComponentBeginOverlap(Box)
  (params (OverlappedComponent :type Primitive%20Component%20Object%20Reference) (OtherActor :type Actor%20Object%20Reference) (OtherComp :type Primitive%20Component%20Object%20Reference) (OtherBodyIndex :type Integer) (bFromSweep :type Boolean) (SweepResult :type Hit%20Result%20Structure%20%28by%20ref%29))
  (if (== OtherActor (Game|GetPlayerCharacter 0))
    (Utilities|FlowControl|DoOnce false
      (:Completed
        (Audio|PlaySound2D "/Game/MainLevel/Sounds/Sound_Spawn.Sound_Spawn" 1.0 1.0 0.0 0 0)
        (Utilities|FlowControl|Delay 0.5)
        (for _array_element (Variables|SpawnSetup|GetEnemyStructure)
          (Game|SpawnActorfromClass (.EnemyClass (Utilities|Struct|BreakEnemyStructur _array_element)) (Transformation|GetActorTransform (.SpawnPoint (Utilities|Struct|BreakEnemyStructur _array_element))) "Undefined" 0 (.BehaviorTree (Utilities|Struct|BreakEnemyStructur _array_element)) (.AssaultPath (Utilities|Struct|BreakEnemyStructur _array_element)) (.WeaponType (Utilities|Struct|BreakEnemyStructur _array_element)) 0))))))

(fn ConstructionScript)